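; Player controller that streams voxel chunk actors around the player pawn on a grid sized from voxel size and elements per chunk.
; Each Tick it updates the pawn's chunk coordinates, then removes and adds chunks without waiting for a cell change.
; Both passes filter by CheckRadius, whose graph holds an unconnected render-range distance test.
; Parallel coordinate and actor arrays track spawned chunks, preventing duplicates and locating those to destroy.
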(event EventBeginPlay
  (CallFunction|Initialize))

(event EventTick
  (params (DeltaSeconds :type Float%20%28single-precision%29))
  (CallFunction|UpdatePosition)
  (CallFunction|RemoveChunk)
  (CallFunction|AddChunk))

(fn ConstructionScript)

(fn Initialize
  (bind _output_get (Variables|ChunkParamentrs|SetchunkSize (* (Variables|Settings|GetchunkLineElements) (Variables|Settings|GetvoxelSize))))
  (Variables|ChunkParamentrs|SetchunkSizeHalf (/ _output_get 2)))

(fn UpdatePosition
  (bind _chunksize (Variables|ChunkParamentrs|GetchunkSize))
  (bind _returnvalue (Math|Conversions|ToFloat(Integer) _chunksize))
  (bind _output_get (Variables|ChunkParamentrs|SetcharecterPosition (* (Transformation|GetActorLocation (Game|Player|GetPlayerPawn 0)) "1.000000,1.000000,0.000000")))
  (if (or (!= (Variables|ChunkParamentrs|GetchunkX) (Math|Float|Floor (/ (.X (Math|Vector|BreakVector _output_get)) _returnvalue))) (!= (Math|Float|Floor (/ (.Y (Math|Vector|BreakVector _output_get)) _returnvalue)) (Variables|ChunkParamentrs|GetchunkY)))
    (Variables|ChunkParamentrs|SetchunkX (Math|Float|Floor (/ (.X (Math|Vector|BreakVector _output_get)) _returnvalue)))
    (Variables|ChunkParamentrs|SetchunkY (Math|Float|Floor (/ (.Y (Math|Vector|BreakVector _output_get)) _returnvalue)))
    (return true)
    (else
      (return false))))

(fn AddChunk
  (bind _chunksize (Variables|ChunkParamentrs|GetchunkSize))
  (bind _chunksizehalf (Variables|ChunkParamentrs|GetchunkSizeHalf))
  (bind _chunkcords (Variables|ChunkParamentrs|GetchunkCords))
  (bind _randerrange (Variables|Settings|GetranderRange))
  (bind _returnvalue (Math|Conversions|ToFloat(Integer) _chunksizehalf))
  (bind _returnvalue_2 (Math|Conversions|ToFloat(Integer) _chunksize))
  (bind _returnvalue_3 (* _randerrange -1))
  (for _index (range _returnvalue_3 _randerrange) ; x
    (for _index_2 (range _returnvalue_3 _randerrange) ; y
      (if (Utilities|CheckRadius (+ (* (+ _index (Variables|ChunkParamentrs|GetchunkX)) _returnvalue_2) _returnvalue) (+ (* (+ _index_2 (Variables|ChunkParamentrs|GetchunkY)) _returnvalue_2) _returnvalue))
        (if (not (Utilities|Array|ContainsItem _chunkcords (Math|Vector2D|MakeVector2D (Math|Conversions|ToFloat(Integer) (+ _index (Variables|ChunkParamentrs|GetchunkX))) (Math|Conversions|ToFloat(Integer) (+ _index_2 (Variables|ChunkParamentrs|GetchunkY))))))
          (Utilities|Array|Add _chunkcords (Math|Vector2D|MakeVector2D (Math|Conversions|ToFloat(Integer) (+ _index (Variables|ChunkParamentrs|GetchunkX))) (Math|Conversions|ToFloat(Integer) (+ _index_2 (Variables|ChunkParamentrs|GetchunkY)))))
          (Development|PrintString (Utilities|String|ToString(Vector) (Math|Vector|MakeVector (* (+ _index (Variables|ChunkParamentrs|GetchunkX)) _returnvalue_2) (* (+ _index_2 (Variables|ChunkParamentrs|GetchunkY)) _returnvalue_2) 0.0)))
          (bind _returnvalue_4 (Game|SpawnActorfromClass "/Game/Voxel/VoxelTestActor_BP.VoxelTestActor_BP_C" (Math|Conversions|ToTransform(Vector) (Math|Vector|MakeVector (* (+ _index (Variables|ChunkParamentrs|GetchunkX)) _returnvalue_2) (* (+ _index_2 (Variables|ChunkParamentrs|GetchunkY)) _returnvalue_2) 0.0)) "Undefined" 0 0))
          (Utilities|Array|Add (Variables|ChunkParamentrs|Getchunks) _returnvalue_4))))))

(fn RemoveChunk
  (bind _chunksize (Variables|ChunkParamentrs|GetchunkSize))
  (bind _chunksizehalf (Variables|ChunkParamentrs|GetchunkSizeHalf))
  (bind _chunks (Variables|ChunkParamentrs|Getchunks))
  (bind _returnvalue (Math|Conversions|ToFloat(Integer) _chunksizehalf))
  (for (_array_element _array_index) (Variables|ChunkParamentrs|GetchunkCords)
    (if (not (Utilities|CheckRadius (+ (* _chunksize (.X (Math|Vector2D|BreakVector2D _array_element))) _returnvalue) (+ (* _chunksize (.Y (Math|Vector2D|BreakVector2D _array_element))) _returnvalue)))
      (Actor|DestroyActor (Utilities|Array|Get(acopy) _chunks _array_index))
      (Utilities|Array|RemoveIndex (Variables|ChunkParamentrs|GetchunkCords) _array_index)
      (Utilities|Array|RemoveIndex _chunks _array_index))))