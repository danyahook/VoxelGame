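; Voxel world actor that spawns decorative props (grass, flowers, saplings, mushrooms, particle effects) and collectible skulls.
; AddInstanceVoxel negates MeshType to select an instanced mesh component or a new particle component, placing it half the player controller's VoxelSize below the given location.
; Skull overlaps remove the instance at the sweep's HitItem, increment the controller's SkullCounter and update its skull widget.
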(event OnComponentBeginOverlap(skull)
  (params (OverlappedComponent :type Primitive%20Component%20Object%20Reference) (OtherActor :type Actor%20Object%20Reference) (OtherComp :type Primitive%20Component%20Object%20Reference) (OtherBodyIndex :type Integer) (bFromSweep :type Boolean) (SweepResult :type Hit%20Result%20Structure%20%28by%20ref%29))
  (bind _asvoxel_player_controller_bp (Utilities|Casting|CastToVoxelPlayerController_BP (Game|GetPlayerController 0)))
  (Class|InstancedStaticMeshComponent|RemoveInstance (Variables|Default|Getskull) (.HitItem (Collision|BreakHitResult SweepResult)))
  (Variables|/Game/Voxel/VoxelPlayerController_BP.VoxelPlayerController_BP_C|SetskullCounter _asvoxel_player_controller_bp (+ (Variables|/Game/Voxel/VoxelPlayerController_BP.VoxelPlayerController_BP_C|GetskullCounter _asvoxel_player_controller_bp) 1))
  (Default|AddSkull (Variables|/Game/Voxel/VoxelPlayerController_BP.VoxelPlayerController_BP_C|GetskullWidget _asvoxel_player_controller_bp)))

(event EventBeginPlay)

(event Collision|EventActorBeginOverlap
  (params (OtherActor :type Actor%20Object%20Reference)))

(event EventTick
  (params (DeltaSeconds :type Float%20%28single-precision%29)))

(event EventAddInstanceVoxel
  (params (instanceLocation :type Vector :default "0, 0, 0") (meshType :type Integer))
  (bind (_x _y _z) (Math|Vector|BreakVector instanceLocation))
  (bind _asvoxel_player_controller_bp (Utilities|Casting|CastToVoxelPlayerController_BP (Game|GetPlayerController 0)))
  (switch int (* meshType -1)
    (:1
      (Components|InstancedStaticMesh|AddInstance (Variables|Default|Getgrass) (Math|Conversions|ToTransform(Vector) (Math|Vector|MakeVector _x _y (- _z (Math|Conversions|ToFloat(Integer) (/ (Variables|/Game/Voxel/VoxelPlayerController_BP.VoxelPlayerController_BP_C|GetvoxelSize _asvoxel_player_controller_bp) 2)))))))
    (:2
      (Components|InstancedStaticMesh|AddInstance (Variables|Default|Getflower) (Math|Conversions|ToTransform(Vector) (Math|Vector|MakeVector _x _y (- _z (Math|Conversions|ToFloat(Integer) (/ (Variables|/Game/Voxel/VoxelPlayerController_BP.VoxelPlayerController_BP_C|GetvoxelSize _asvoxel_player_controller_bp) 2)))))))
    (:3
      (Components|InstancedStaticMesh|AddInstance (Variables|Default|Getflower_1) (Math|Conversions|ToTransform(Vector) (Math|Vector|MakeVector _x _y (- _z (Math|Conversions|ToFloat(Integer) (/ (Variables|/Game/Voxel/VoxelPlayerController_BP.VoxelPlayerController_BP_C|GetvoxelSize _asvoxel_player_controller_bp) 2)))))))
    (:4
      (Components|InstancedStaticMesh|AddInstance (Variables|Default|Getsapling) (Math|Conversions|ToTransform(Vector) (Math|Vector|MakeVector _x _y (- _z (Math|Conversions|ToFloat(Integer) (/ (Variables|/Game/Voxel/VoxelPlayerController_BP.VoxelPlayerController_BP_C|GetvoxelSize _asvoxel_player_controller_bp) 2)))))))
    (:5
      (Components|InstancedStaticMesh|AddInstance (Variables|Default|Getmushroom) (Math|Conversions|ToTransform(Vector) (Math|Vector|MakeVector _x _y (- _z (Math|Conversions|ToFloat(Integer) (/ (Variables|/Game/Voxel/VoxelPlayerController_BP.VoxelPlayerController_BP_C|GetvoxelSize _asvoxel_player_controller_bp) 2)))))))
    (:6
      (Components|InstancedStaticMesh|AddInstance (Variables|Default|Getmushroom1) (Math|Conversions|ToTransform(Vector) (Math|Vector|MakeVector _x _y (- _z (Math|Conversions|ToFloat(Integer) (/ (Variables|/Game/Voxel/VoxelPlayerController_BP.VoxelPlayerController_BP_C|GetvoxelSize _asvoxel_player_controller_bp) 2)))))))
    (:7
      (AddComponent|AddParticleSystemComponent false (Math|Conversions|ToTransform(Vector) (Math|Vector|MakeVector _x _y (- _z (Math|Conversions|ToFloat(Integer) (/ (Variables|/Game/Voxel/VoxelPlayerController_BP.VoxelPlayerController_BP_C|GetvoxelSize _asvoxel_player_controller_bp) 2)))))))
    (:8
      (Components|InstancedStaticMesh|AddInstance (Variables|Default|Getskull) (Math|Conversions|ToTransform(Vector) (Math|Vector|MakeVector _x _y (- _z (Math|Conversions|ToFloat(Integer) (/ (Variables|/Game/Voxel/VoxelPlayerController_BP.VoxelPlayerController_BP_C|GetvoxelSize _asvoxel_player_controller_bp) 2)))))))))

(fn ConstructionScript)